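; BP_ClownFinal is a clown enemy that constantly advances along its forward vector and laughs every few seconds.
; Movement is a self-calling event with a tiny delay that offsets the actor's location without sweep.
; A looping timer checks player distance and slows the clown when the player is near.
; Overlapping its Detection component with a BPI_Player actor deals massive damage and stops the movement.
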(event OnComponentBeginOverlap(Detection)
  (params (OverlappedComponent :type Primitive%20Component%20Object%20Reference) (OtherActor :type Actor%20Object%20Reference) (OtherComp :type Primitive%20Component%20Object%20Reference) (OtherBodyIndex :type Integer) (bFromSweep :type Boolean) (SweepResult :type Hit%20Result%20Structure%20%28by%20ref%29))
  (if (Utilities|DoesObjectImplementInterface OtherActor "/Game/Player/BPI_Player.BPI_Player_C")
    (Class|BPIPlayer|GetDamage(Message) OtherActor 2.5e+03)
    (Variables|Default|SetCanMove false)))

(event Custom|MoveForward
  (if (Variables|Default|GetCanMove)
    (Transformation|SetActorLocation (+ (Transformation|GetActorLocation) (* (Transformation|GetActorForwardVector) (Variables|Default|GetVelocity))) false false)
    (Utilities|FlowControl|Delay 0.001)
    (CallFunction|MoveForward)))

(event Custom|Laugh
  (Audio|Components|Audio|Play (Variables|Default|GetFinalClown) 0.0)
  (Utilities|FlowControl|Delay (Math|Random|RandomFloatinRange 5.0 7.0))
  (CallFunction|Laugh))

(event EventBeginPlay
  (CallFunction|MoveForward)
  (Utilities|Time|SetTimerbyFunctionName 0 "PlayerDistance" 0.001 true)
  (CallFunction|Laugh))

(fn ConstructionScript)

(fn PlayerDistance
  (if (< (Math|Vector|Distance(Vector) (Transformation|GetActorLocation) (Transformation|GetActorLocation (Game|GetPlayerCharacter 0))) 6e+02)
    (Variables|Default|SetVelocity 2.5)
    (else
      (Variables|Default|SetVelocity 8.0))))