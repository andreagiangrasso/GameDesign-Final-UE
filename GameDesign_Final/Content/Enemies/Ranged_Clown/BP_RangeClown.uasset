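; Ranged clown enemy that, once the player enters its detection volume, turns to face them, cranks its lever and repeatedly plays an attack montage.
; Self-recursive delayed events drive these loops; PlayerOnSight never clears, as end overlap also sets it true.
; RangeAttack spawns projectiles; debounced Damage decrements Life until death triggers animation, physics and a flying lever.
; A second volume toggles the player's interact prompt, with interaction opening a W_ChangeTo widget.
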(event OnComponentBeginOverlap(DetectPlayer)
  (params (OverlappedComponent :type Primitive%20Component%20Object%20Reference) (OtherActor :type Actor%20Object%20Reference) (OtherComp :type Primitive%20Component%20Object%20Reference) (OtherBodyIndex :type Integer) (bFromSweep :type Boolean) (SweepResult :type Hit%20Result%20Structure%20%28by%20ref%29))
  (if (Utilities|DoesObjectImplementInterface OtherActor "/Game/Player/BPI_Player.BPI_Player_C")
    (Variables|Control|SetPlayerOnSight true)
    (CallFunction|RotateLever)
    (CallFunction|LookatPlayer)
    (Utilities|FlowControl|Delay 2.0)
    (CallFunction|Attack)))

(event OnComponentBeginOverlap(CollisionToChange)
  (params (OverlappedComponent :type Primitive%20Component%20Object%20Reference) (OtherActor :type Actor%20Object%20Reference) (OtherComp :type Primitive%20Component%20Object%20Reference) (OtherBodyIndex :type Integer) (bFromSweep :type Boolean) (SweepResult :type Hit%20Result%20Structure%20%28by%20ref%29))
  (if (Utilities|DoesObjectImplementInterface OtherActor "/Game/Player/BPI_Player.BPI_Player_C")
    (Class|BPIInteract|EnabledInteract(Message) OtherActor self)))

(event OnComponentEndOverlap(CollisionToChange)
  (params (OverlappedComponent :type Primitive%20Component%20Object%20Reference) (OtherActor :type Actor%20Object%20Reference) (OtherComp :type Primitive%20Component%20Object%20Reference) (OtherBodyIndex :type Integer))
  (if (Utilities|DoesObjectImplementInterface OtherActor "/Game/Player/BPI_Player.BPI_Player_C")
    (Class|BPIInteract|DisabledInteract(Message) OtherActor)))

(event OnComponentEndOverlap(DetectPlayer)
  (params (OverlappedComponent :type Primitive%20Component%20Object%20Reference) (OtherActor :type Actor%20Object%20Reference) (OtherComp :type Primitive%20Component%20Object%20Reference) (OtherBodyIndex :type Integer))
  (if (Utilities|DoesObjectImplementInterface OtherActor "/Game/Player/BPI_Player.BPI_Player_C")
    (Variables|Control|SetPlayerOnSight true)))

(event Custom|RotateLever
  (if (and (Variables|Control|GetIsAlive) (Variables|Control|GetPlayerOnSight))
    (Transformation|AddRelativeRotation (Variables|Default|GetClown_Lever) "0, 0,1.000000" false false)
    (Utilities|FlowControl|Delay 0.001)
    (CallFunction|RotateLever)))

(event Custom|LeverFly
  (bind _clown_lever (Variables|Default|GetClown_Lever))
  (Physics|SetSimulatePhysics _clown_lever true)
  (Class|PrimitiveComponent|AddForceatLocationLocal _clown_lever "0.000000,2500.000000,300.000000" "0, 0, 0" "None"))

(event Custom|Die
  (bind _mesh (Variables|Character|GetMesh))
  (bind _mesh_2 (Variables|Character|GetMesh))
  (Variables|Control|SetIsAlive false)
  (Components|Animation|SetAnimationMode _mesh "AnimationSingleNode")
  (Components|Animation|PlayAnimation _mesh "/Game/Enemies/Ranged_Clown/Anims/Head_Death.Head_Death" false)
  (Collision|SetCollisionResponsetoChannel (Variables|Collision|GetCapsuleComponent) "ECC_Pawn" "ECR_Ignore")
  (Utilities|FlowControl|Delay 1.0)
  (Physics|SetSimulatePhysics _mesh_2 true)
  (Physics|AddForce _mesh_2 "0, 0,50.000000" "None" false)
  (CallFunction|LeverFly)
  (Collision|SetCollisionEnabled (Variables|Default|GetCollisionToChange) "QueryOnly"))

(event Custom|LookAtPlayer
  (bind _mesh (Variables|Character|GetMesh))
  (if (and (Variables|Control|GetIsAlive) (Variables|Control|GetPlayerOnSight))
    (Transformation|SetWorldRotation _mesh (Math|Rotator|MakeRotator 0.0 0.0 (- (.yaw (Math|Rotator|FindLookatRotation (Transformation|GetWorldLocation _mesh) (Transformation|GetWorldLocation (Variables|/Script/Engine.Character|GetMesh (Game|GetPlayerCharacter 0))))) 9e+01)) false false)
    (Utilities|FlowControl|Delay 0.1)
    (CallFunction|LookatPlayer)))

(event Custom|Attack
  (if (and (Variables|Control|GetIsAlive) (Variables|Control|GetPlayerOnSight))
    (Animation|PlayAnimMontage "/Game/Enemies/Ranged_Clown/Anims/Head_Attack_Montage.Head_Attack_Montage" 1.0 "None")
    (Utilities|FlowControl|Delay 4.0)
    (CallFunction|Attack)))

(event EventBeginPlay)

(event Collision|EventActorBeginOverlap
  (params (OtherActor :type Actor%20Object%20Reference)))

(event EventDoInteraction
  (bind _returnvalue (UserInterface|CreateWidget "/Game/Interactables/ChangeTo/W_ChangeTo.W_ChangeTo_C" 0 self))
  (UserInterface|Viewport|AddtoViewport _returnvalue 0))

(event EventDamage
  (if (Variables|Control|GetIsAlive)
    (Utilities|FlowControl|DoOnce false :!label _label
      (:Completed
        (Utilities|FlowControl|Sequence
          (:then_0
            (Math|Integer|DecrementInt (Variables|Control|GetLife)
              (:%20%20
                (if (<= (Variables|Control|GetLife) 0)
                  (CallFunction|Die)))))
          (:then_1
            (Utilities|FlowControl|Delay 0.2)
            (goto _label Reset)))))))

(event EventRangeAttack
  (bind _self self)
  (Game|SpawnActorfromClass "/Game/Enemies/Ranged_Clown/Proyectile/BP_Projectile.BP_Projectile_C" (Math|Transform|MakeTransform (Transformation|GetWorldLocation (Variables|Default|GetSpawnPoint)) (Math|Rotator|MakeRotator 0.0 0.0 (+ (.yaw (Transformation|GetWorldRotation (Variables|Character|GetMesh))) 9e+01)) "1,1,1") "Undefined" _self _self))

(fn ConstructionScript)