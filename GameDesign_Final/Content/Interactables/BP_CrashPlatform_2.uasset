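; Interactable platform that slides its cube between the Init and End positions each time the player interacts with it.
; DoInteraction uses a FlipFlop to alternately play and reverse the Move timeline, which lerps the cube's relative location.
; Player input is disabled when movement starts and restored when the timeline finishes.
; The Detection volume enables and disables the interact message on overlapping actors that implement BPI_Player.
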(event OnComponentBeginOverlap(Detection)
  (params (OverlappedComponent :type Primitive%20Component%20Object%20Reference) (OtherActor :type Actor%20Object%20Reference) (OtherComp :type Primitive%20Component%20Object%20Reference) (OtherBodyIndex :type Integer) (bFromSweep :type Boolean) (SweepResult :type Hit%20Result%20Structure%20%28by%20ref%29))
  (if (Utilities|DoesObjectImplementInterface OtherActor "/Game/Player/BPI_Player.BPI_Player_C")
    (Class|BPIInteract|EnabledInteract(Message) OtherActor self)))

(event OnComponentEndOverlap(Detection)
  (params (OverlappedComponent :type Primitive%20Component%20Object%20Reference) (OtherActor :type Actor%20Object%20Reference) (OtherComp :type Primitive%20Component%20Object%20Reference) (OtherBodyIndex :type Integer))
  (if (Utilities|DoesObjectImplementInterface OtherActor "/Game/Player/BPI_Player.BPI_Player_C")
    (Class|BPIInteract|DisabledInteract(Message) OtherActor)))

(event EventBeginPlay)

(event Collision|EventActorBeginOverlap
  (params (OtherActor :type Actor%20Object%20Reference)))

(event EventTick
  (params (DeltaSeconds :type Float%20%28single-precision%29)))

(event EventDoInteraction
  (Input|DisableInput (Game|GetPlayerCharacter 0) (Game|GetPlayerController 0))
  (Utilities|FlowControl|FlipFlop
    (:A
      (bind _newtrack_0 (Timeline|Move Play)
        (:Update
          (Transformation|SetRelativeLocation (Variables|Default|GetCube) (Math|Vector|Lerp(Vector) (Variables|/Script/Engine.SceneComponent|GetRelativeLocation (Variables|Default|GetInit)) (Variables|/Script/Engine.SceneComponent|GetRelativeLocation (Variables|Default|GetEnd)) _newtrack_0) false false))
        (:Finished
          (Input|EnableInput (Game|GetPlayerCharacter 0) (Game|GetPlayerController 0)))))
    (:B
      (Timeline|Move Reverse))))

(fn ConstructionScript)