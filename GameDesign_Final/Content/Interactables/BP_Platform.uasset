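; BP_Platform is an interactable platform that slides its Cube between the Init and End scene points.
; Move plays the MovePlatform timeline, which lerps the Cube's world location between the two points, and GoBack reverses it.
; The first update spawns a 2D movement sound, guarded by a flag, and the timeline's finish fades it out.
; RefreshInitialPosition snaps the Cube back to Init.
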(event Custom|Move
  (bind _newtrack_0 (Timeline|MovePlatform Play)
    (:Update
      (Transformation|SetWorldLocation (Variables|Default|GetCube) (Math|Vector|Lerp(Vector) (Transformation|GetWorldLocation (Variables|Default|GetInit)) (Transformation|GetWorldLocation (Variables|Default|GetEnd)) _newtrack_0) false false)
      (if (not (Variables|Default|GetSoundPlaying))
        (Variables|Default|SetSoundPlaying true)
        (bind _returnvalue (Audio|SpawnSound2D "/Game/Sounds/Platform_Movement.Platform_Movement" 1.0 1.0 0.0 0))
        (Variables|Default|SetSound _returnvalue)))
    (:Finished
      (bind _sound (Variables|Default|GetSound)
        (:then
          (Audio|Components|Audio|FadeOut _sound 0.02 0.0 "Linear" :!class /Script/Engine.AudioComponent)
          (Variables|Default|SetSoundPlaying false))
        (:else)))))

(event Custom|RefreshInitialPosition
  (Transformation|SetWorldLocation (Variables|Default|GetCube) (Transformation|GetWorldLocation (Variables|Default|GetInit)) false false))

(event Custom|GoBack
  (bind _newtrack_0 (Timeline|MovePlatform Reverse)
    (:Update
      (Transformation|SetWorldLocation (Variables|Default|GetCube) (Math|Vector|Lerp(Vector) (Transformation|GetWorldLocation (Variables|Default|GetInit)) (Transformation|GetWorldLocation (Variables|Default|GetEnd)) _newtrack_0) false false)
      (if (not (Variables|Default|GetSoundPlaying))
        (Variables|Default|SetSoundPlaying true)
        (bind _returnvalue (Audio|SpawnSound2D "/Game/Sounds/Platform_Movement.Platform_Movement" 1.0 1.0 0.0 0))
        (Variables|Default|SetSound _returnvalue)))
    (:Finished
      (bind _sound (Variables|Default|GetSound)
        (:then
          (Audio|Components|Audio|FadeOut _sound 0.02 0.0 "Linear" :!class /Script/Engine.AudioComponent)
          (Variables|Default|SetSoundPlaying false))
        (:else)))))

(fn ConstructionScript)