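; BP_ClimbedRope_2 is an interactable climbed-rope actor that prompts player interaction when approached.
; Its Box overlap events tell actors implementing BPI_Player to show or hide the interact message, passing itself as the target on entry.
; DoInteraction runs once through a DoOnce gate and calls CallFearCord.
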(event OnComponentBeginOverlap(Box)
  (params (OverlappedComponent :type Primitive%20Component%20Object%20Reference) (OtherActor :type Actor%20Object%20Reference) (OtherComp :type Primitive%20Component%20Object%20Reference) (OtherBodyIndex :type Integer) (bFromSweep :type Boolean) (SweepResult :type Hit%20Result%20Structure%20%28by%20ref%29))
  (if (Utilities|DoesObjectImplementInterface OtherActor "/Game/Player/BPI_Player.BPI_Player_C")
    (Class|BPIInteract|EnabledInteract(Message) OtherActor self)))

(event OnComponentEndOverlap(Box)
  (params (OverlappedComponent :type Primitive%20Component%20Object%20Reference) (OtherActor :type Actor%20Object%20Reference) (OtherComp :type Primitive%20Component%20Object%20Reference) (OtherBodyIndex :type Integer))
  (if (Utilities|DoesObjectImplementInterface OtherActor "/Game/Player/BPI_Player.BPI_Player_C")
    (Class|BPIInteract|DisabledInteract(Message) OtherActor)))

(event EventDoInteraction
  (Utilities|FlowControl|DoOnce false
    (:Completed
      (Default|CallFearCord))))

(fn ConstructionScript)