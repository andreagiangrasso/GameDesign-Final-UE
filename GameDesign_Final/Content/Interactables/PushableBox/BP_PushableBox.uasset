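; BP_PushableBox is a physics box that holds off simulating until no player overlaps it, presumably to avoid spawning inside them.
; On BeginPlay the mesh ignores Pawns, then waits briefly before activation.
; The Control component's overlaps flag BPI_Player actors, and activation polls that flag in a delay loop.
; Once clear, the mesh simulates physics, blocks Pawns and switches object type, and Control collision turns off.
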(event OnComponentBeginOverlap(Control)
  (params (OverlappedComponent :type Primitive%20Component%20Object%20Reference) (OtherActor :type Actor%20Object%20Reference) (OtherComp :type Primitive%20Component%20Object%20Reference) (OtherBodyIndex :type Integer) (bFromSweep :type Boolean) (SweepResult :type Hit%20Result%20Structure%20%28by%20ref%29))
  (if (Utilities|DoesObjectImplementInterface OtherActor "/Game/Player/BPI_Player.BPI_Player_C")
    (Variables|Default|SetPlayerIn true)))

(event OnComponentEndOverlap(Control)
  (params (OverlappedComponent :type Primitive%20Component%20Object%20Reference) (OtherActor :type Actor%20Object%20Reference) (OtherComp :type Primitive%20Component%20Object%20Reference) (OtherBodyIndex :type Integer))
  (if (Utilities|DoesObjectImplementInterface OtherActor "/Game/Player/BPI_Player.BPI_Player_C")
    (Variables|Default|SetPlayerIn false)))

(event Custom|ActivatePhysics
  (bind _staticmesh (Variables|Default|GetStaticMesh))
  (if (Variables|Default|GetPlayerIn) :!label _label
    (Utilities|FlowControl|Delay 0.2)
    (goto _label)
    (else
      (Physics|SetSimulatePhysics (Variables|Default|GetStaticMesh) true)
      (Collision|SetCollisionEnabled (Variables|Default|GetControl) "NoCollision")
      (Collision|SetCollisionResponsetoChannel _staticmesh "ECC_Pawn" "ECR_Block")
      (Collision|SetCollisionObjectType _staticmesh "ECC_GameTraceChannel1"))))

(event EventBeginPlay
  (bind _staticmesh (Variables|Default|GetStaticMesh))
  (Collision|SetCollisionResponsetoChannel _staticmesh "ECC_Pawn" "ECR_Ignore")
  (Collision|SetCollisionObjectType _staticmesh "ECC_WorldDynamic")
  (Utilities|FlowControl|Delay 1.0)
  (CallFunction|ActivatePhysics))

(fn ConstructionScript)