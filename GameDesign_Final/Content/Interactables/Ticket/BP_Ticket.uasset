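; BP_Ticket is a pickup that awards a quantity of tickets to the player.
; When PlayerDetect is overlapped, it asks the other actor whether it is the player, then sends it Quantity through GetTicketMessage once, disables collision and destroys itself.
; A Movement timeline that would move TicketModel between InitialPos and EndPos is present but never runs.
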(event OnComponentBeginOverlap(PlayerDetect)
  (params (OverlappedComponent :type Primitive%20Component%20Object%20Reference) (OtherActor :type Actor%20Object%20Reference) (OtherComp :type Primitive%20Component%20Object%20Reference) (OtherBodyIndex :type Integer) (bFromSweep :type Boolean) (SweepResult :type Hit%20Result%20Structure%20%28by%20ref%29))
  (bind _yes_no (Class|BPIPlayer|IsPlayer(Message) OtherActor))
  (if _yes_no
    (Utilities|FlowControl|DoOnce false
      (:Completed
        (Class|BPIPlayer|GetTicket(Message) OtherActor (Variables|Default|GetQuantity))
        (Collision|SetActorEnableCollision false)
        (Actor|DestroyActor)))))

(event EventBeginPlay)

(fn ConstructionScript)